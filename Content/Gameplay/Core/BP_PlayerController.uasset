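; Player controller that maps Enhanced Input actions to the first pawn for movement, camera look, interaction and pausing.
; BeginPlay adds the default mapping context and caches the player character, which receives left-click input as interact logic.
; Look input scales by a sensitivity modifier with inverted pitch, and movement follows the pawn's forward and right vectors.
; Pause toggles the gameplay manager's state between Gameplay and Paused and notifies the character.
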(event Input|EnhancedActionEvents|EnhancedInputActionIA_Move
  (params (ActionValue :type Vector%202D%20Structure) (ElapsedSeconds :type Float%20%28double-precision%29) (TriggeredSeconds :type Float%20%28double-precision%29) (InputAction :type Input%20Action%20Object%20Reference :default "/Game/Gameplay/Input/IA_Move.IA_Move"))
  (bind _returnvalue (Game|Player|GetPlayerPawn 0))
  (Pawn|Input|AddMovementInput _returnvalue (+ (* (Transformation|GetActorForwardVector _returnvalue) (.x ActionValue)) (* (Transformation|GetActorRightVector _returnvalue) (.y ActionValue))) 1.0 false))

(event Input|EnhancedActionEvents|EnhancedInputActionIA_MoveCamera
  (params (ActionValue :type Vector%202D%20Structure) (ElapsedSeconds :type Float%20%28double-precision%29) (TriggeredSeconds :type Float%20%28double-precision%29) (InputAction :type Input%20Action%20Object%20Reference :default "/Game/Gameplay/Input/IA_MoveCamera.IA_MoveCamera"))
  (bind _returnvalue (Game|Player|GetPlayerPawn 0))
  (Pawn|Input|AddControllerPitchInput _returnvalue (* (* (.y ActionValue) -1.0) (Variables|Default|GetSensitivity%20Modifier)))
  (Pawn|Input|AddControllerYawInput _returnvalue (* (.x ActionValue) (Variables|Default|GetSensitivity%20Modifier))))

(event Input|EnhancedActionEvents|EnhancedInputActionIA_LMB
  (params (ActionValue :type Boolean) (ElapsedSeconds :type Float%20%28double-precision%29) (TriggeredSeconds :type Float%20%28double-precision%29) (InputAction :type Input%20Action%20Object%20Reference :default "/Game/Gameplay/Input/IA_LMB.IA_LMB"))
  (Default|StartInteractLogic (Variables|Default|GetCached%20Player) ActionValue))

(event Input|EnhancedActionEvents|EnhancedInputActionIA_Pause
  (params (ActionValue :type Boolean) (ElapsedSeconds :type Float%20%28double-precision%29) (TriggeredSeconds :type Float%20%28double-precision%29) (InputAction :type Input%20Action%20Object%20Reference :default "/Game/Gameplay/Input/IA_Pause.IA_Pause"))
  (bind _asbp_player_character (Utilities|Casting|CastToBP_PlayerCharacter (Game|Player|GetPlayerPawn 0)))
  (bind _returnvalue (Actor|GetActorOfClass "/Game/Gameplay/GameplayManager/BP_GameplayManager.BP_GameplayManager_C"))
  (switch Utilities|FlowControl|Switch|SwitchonE_GameState (Variables|/Game/Gameplay/GameplayManager/BP_GameplayManager.BP_GameplayManager_C|GetGame%20State _returnvalue)
    (:NewEnumerator1
      (Variables|/Game/Gameplay/GameplayManager/BP_GameplayManager.BP_GameplayManager_C|SetGame%20State _returnvalue "NewEnumerator2")
      (Default|CallOnGamePaused _asbp_player_character true))
    (:NewEnumerator2
      (Variables|/Game/Gameplay/GameplayManager/BP_GameplayManager.BP_GameplayManager_C|SetGame%20State _returnvalue "NewEnumerator1")
      (Default|CallOnGamePaused _asbp_player_character false))))

(event EventBeginPlay
  (Input|AddMappingContext (PlayerController|LocalPlayerSubsystems|GetEnhancedInputLocalPlayerSubsystem) "/Game/Gameplay/Input/IMC_Default.IMC_Default" 0 "(bIgnoreAllPressedKeysUntilRelease=True,bForceImmediately=False,bNotifyUserSettings=False)")
  (bind _asbp_player_character (Utilities|Casting|CastToBP_PlayerCharacter (Game|Player|GetPlayerPawn 0)))
  (Variables|Default|SetCached%20Player _asbp_player_character))

(event EventTick
  (params (DeltaSeconds :type Float%20%28single-precision%29)))

(fn ConstructionScript)