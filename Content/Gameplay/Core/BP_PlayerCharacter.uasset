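; Player character that detects, picks up and holds interactable items (plushies) in front of the camera.
; StartInteractLogic traces for BPI_Interactable actors on press and drops on release, using start/stop events to notify the item.
; Each Tick updates hover state, broadcasting changes, and moves the held item to face the camera.
; A second trace keeps the hold point offset from blocking surfaces, with an optional debug sphere.
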(event Custom|Start%20Holding%20Item
  (Variables|Interaction|SetIs%20Holding%20Item true)
  (bind _asbpi_interactable (Utilities|Casting|CastToBPI_Interactable (Variables|Interaction|GetHeld%20Item)))
  (Default|StartHolding _asbpi_interactable self))

(event Custom|Stop%20Holding%20Item
  (Variables|Interaction|SetIs%20Holding%20Item false)
  (bind _asbpi_interactable (Utilities|Casting|CastToBPI_Interactable (Variables|Interaction|GetHeld%20Item)))
  (Default|StopHolding _asbpi_interactable self)
  (Variables|Interaction|SetHeld%20Item 0))

(event EventBeginPlay
  (Utilities|FlowControl|Sequence
    (:then_0
      (EventDispatchers|BindEventtoOnItemStartHolding (delegate Custom|Start%20Holding%20Item)))
    (:then_1
      (EventDispatchers|BindEventtoOnItemStopHolding (delegate Custom|Stop%20Holding%20Item)))))

(event Collision|EventActorBeginOverlap
  (params (OtherActor :type Actor%20Object%20Reference)))

(event EventTick
  (params (DeltaSeconds :type Float%20%28single-precision%29))
  (CallFunction|WallLocationFindLogic)
  (CallFunction|CheckforInteractableHover)
  (CallFunction|SetHeldActorTransform)
  ;[0.1316 0.3627 0.5521 0.5] Debug Interaction trace
  (if (Variables|Default|GetIsDebugging)
    (Rendering|Debug|DrawDebugSphere (Variables|WallDetection|GetHold%20Plushie%20Location) 5.0 12 "(R=1.000000,G=1.000000,B=1.000000,A=1.000000)" 0.0 0.25)))

(fn ConstructionScript)

(fn WallLocationFindLogic
  (bind _camera (Variables|Default|GetCamera))
  (bind _camera_2 (Variables|Default|GetCamera))
  (bind _returnvalue (Transformation|GetWorldLocation _camera_2))
  ;[0.1316 0.3627 0.5521 0.5] Trace to find wall
  (bind _outhit (Collision|LineTraceByChannel _returnvalue (+ _returnvalue (* (Math|Vector|GetForwardVector _camera_2) (Variables|WallDetection|GetHold%20Distance))) "TraceTypeQuery1" false (Utilities|Array|MakeArray (Variables|Interaction|GetHeld%20Item)) "None"))
  (if (.bblockinghit _outhit)
    ;[0.1316 0.3627 0.5521 0.5] Find plushie hold location at some distance from wall
    (bind _output_get (Variables|WallDetection|SetLook%20Near%20Wall%20Location (.location _outhit)))
    (Variables|WallDetection|SetHold%20Plushie%20Location (+ (Variables|WallDetection|GetLook%20Near%20Wall%20Location) (* (Math|Vector|Normalize (- (Transformation|GetWorldLocation (Variables|Default|GetCamera)) _output_get)) (Variables|WallDetection|GetHold%20Wall%20Offset%20Distance))))
    (return)
    (else
      ;[0.1316 0.3627 0.5521 0.5] Find plushie hold location if not near wall
      (Variables|WallDetection|SetHold%20Plushie%20Location (+ (Transformation|GetWorldLocation _camera) (* (Math|Vector|GetForwardVector _camera) (- (Variables|WallDetection|GetHold%20Distance) (Variables|WallDetection|GetHold%20Wall%20Offset%20Distance)))))
      (return))))

(fn SetHeldActorTransform
  (bind _held_item (Variables|Interaction|GetHeld%20Item))
  (bind _hold_plushie_location (Variables|WallDetection|GetHold%20Plushie%20Location))
  (if (Variables|Interaction|GetIs%20Holding%20Item)
    (Utilities|IsValid _held_item
      (:Is%20Valid
        (Transformation|SetActorLocation _held_item _hold_plushie_location false false)
        (Transformation|SetActorRotation _held_item (Math|Rotator|FindLookatRotation _hold_plushie_location (Transformation|GetWorldLocation (Variables|Default|GetCamera))))
        (return))
      (:Is%20Not%20Valid
        (return)))
    (else
      (return))))

(fn StartInteractLogic
  (params (Pressed%20LMB :type Boolean))
  (bind _is_holding_item (Variables|Interaction|GetIs%20Holding%20Item))
  (bind _camera (Variables|Default|GetCamera))
  (bind _returnvalue (Transformation|GetWorldLocation _camera))
  (if Pressed%20LMB
    (if (not _is_holding_item)
      (bind _outhit (Collision|LineTraceByChannel _returnvalue (+ _returnvalue (* (Math|Vector|GetForwardVector _camera) (Variables|WallDetection|GetInteract%20Distance))) "TraceTypeQuery1" true 0 "None"))
      (Utilities|Casting|CastToBPI_Interactable (.hitactor _outhit))
      (Variables|Interaction|SetHeld%20Item (.hitactor _outhit))
      (Default|CallOnItemStartHolding))
    (elif _is_holding_item
      (Default|CallOnItemStopHolding))))

(fn CheckforInteractableHover
  (bind _camera (Variables|Default|GetCamera))
  (bind _returnvalue (Transformation|GetWorldLocation _camera))
  ;[0.1316 0.3627 0.5521 0.5] Trace to find wall
  (bind _outhit (Collision|LineTraceByChannel _returnvalue (+ _returnvalue (* (Math|Vector|GetForwardVector _camera) (Variables|WallDetection|GetInteract%20Distance))) "TraceTypeQuery1" true 0 "None"))
  (if (.bblockinghit _outhit)
    (Utilities|Casting|CastToBPI_Interactable (.hitactor _outhit)
      (:then
        (if (not (Variables|Interaction|GetIs%20Hovering%20Item))
          (bind _output_get (Variables|Interaction|SetIs%20Hovering%20Item true))
          (Default|CallOnItemHoverStateChanged _output_get)))
      (:CastFailed
        (if (Variables|Interaction|GetIs%20Hovering%20Item) :!label _label
          (bind _output_get_2 (Variables|Interaction|SetIs%20Hovering%20Item false))
          (Default|CallOnItemHoverStateChanged _output_get_2))))
    (else
      (goto _label))))