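; Gameplay manager that runs a timed plushie-collecting round ending in a quiz.
; On game start it optionally shows the tutorial, shuffles room colors into dynamic materials, gives spawn points random animals and prices, and spawns the chest and player at a random point.
; Plushies turned in at the chest are recorded while a looping timer counts down.
; On timeout it computes answers on prices, rooms, colors and animal traits, then broadcasts them to start questioning.
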(event Custom|Plushie%20Turned%20In_Event
  (params (Plushie%20Gameplay%20Data :type F%20Plushie%20Manager%20Data%20Structure) (Plushie%20Spawn%20Data :type F%20Plushie%20Spawn%20Data%20Structure))
  ;[0.1316 0.3627 0.5521 0.5] Detect plushie turning in
  (Utilities|Array|Add (Variables|Default|GetQuestions%20Data) (Utilities|Struct|MakeF_FullAnimalData Plushie%20Gameplay%20Data Plushie%20Spawn%20Data)))

(event Custom|Start
  (CallFunction|ShowTutorialifNeeded)
  (Utilities|FlowControl|Sequence
    (:then_0
      (CallFunction|SetupDataArrays)
      (CallFunction|SetupRoomColors)
      (CallFunction|SetupPlushiesData)
      (CallFunction|SetupChestDataandPlayerSpawn))
    (:then_1
      ;[0.1316 0.3627 0.5521 0.5] Detect plushie turning in
      (EventDispatchers|AssignPlushieTurnedin (Variables|Runtime|Chest|GetSpawned%20Chest) (delegate Custom|Plushie%20Turned%20In_Event)))
    (:then_2
      ;[0.1316 0.3627 0.5521 0.5] Start generating question answers and choose possible questions to ask player.
      (EventDispatchers|BindEventtoTimerFinished (EventDispatchers|CreateEvent :!event ChooseQuestionsandGenerateAnswers)))
    (:then_3
      ;[0.1316 0.3627 0.5521 0.5] Start timer
      (Variables|Timer|SetCurrent%20Time (Variables|Timer|GetStart%20Time))
      (bind _returnvalue (Utilities|Time|SetTimerbyEvent (EventDispatchers|CreateEvent :!event TickTimer) 0.0001 true true))
      (Variables|Timer|SetTimer%20Handle _returnvalue))))

(event Custom|Timer%20Ran%20Out
  (CallFunction|FindCorrectAnswers)
  (Default|CallOnStartedQuestioning (Variables|Default|GetQuestions%20Data) (Variables|Default|GetCorrectAnswers)))

(event EventBeginPlay
  (Utilities|FlowControl|Sequence
    (:then_0
      (EventDispatchers|BindEventtoOnGameStarted (delegate Custom|Start)))
    (:then_1
      (EventDispatchers|AssignTimerFinished (delegate Custom|Timer%20Ran%20Out)))))

(event Collision|EventActorBeginOverlap
  (params (OtherActor :type Actor%20Object%20Reference)))

(event EventTick
  (params (DeltaSeconds :type Float%20%28single-precision%29)))

(fn ConstructionScript)

(fn GetRandomPrice
  (params (Min :type Integer) (Max :type Integer))
  (return (Math|Random|RandomIntegerinRange Min Max)))

(fn SetupPlushiesData
  (bind _outactors (Actor|GetAllActorsOfClass "/Game/Gameplay/GameplayManager/BP_SpawnPoint.BP_SpawnPoint_C"))
  (for _array_element _outactors
    (bind _output_get (Variables|Runtime|Plushie|SetCurrent%20Animal (.OutItem (Utilities|Array|Random (Variables|CompileTime|Plushie|GetAnimals%20Array)))))
    (bind _animal_data (Default|GetAnimalDatabyType (Variables|CompileTime|Plushie|GetAnimal%20Data) (Variables|Runtime|Plushie|GetCurrent%20Animal)))
    (Variables|Runtime|Plushie|SetCurrent%20Animal%20Data _animal_data)
    (Variables|/Game/Gameplay/GameplayManager/BP_SpawnPoint.BP_SpawnPoint_C|SetPlushie%20Gameplay%20Data _array_element (Utilities|Struct|MakeF_PlushieManagerData (.Value (Utilities|Map|Find (Variables|Runtime|Plushie|GetRoom%20Type%20to%20Color) (.roomtype (Variables|/Game/Gameplay/GameplayManager/BP_SpawnPoint.BP_SpawnPoint_C|GetPlushie%20Spawn%20Data _array_element)))) _output_get (CallFunction|GetRandomPrice (Variables|CompileTime|Plushie|GetMin%20Plushie%20Price) (Variables|CompileTime|Plushie|GetMax%20Plushie%20Price)) (.iscarnivore (Variables|Runtime|Plushie|GetCurrent%20Animal%20Data)) (.isherbivore (Variables|Runtime|Plushie|GetCurrent%20Animal%20Data)) (.isflying (Variables|Runtime|Plushie|GetCurrent%20Animal%20Data)) (.isswimming (Variables|Runtime|Plushie|GetCurrent%20Animal%20Data)) (.name (Variables|Runtime|Plushie|GetCurrent%20Animal%20Data))))
    (Variables|/Game/Gameplay/GameplayManager/BP_SpawnPoint.BP_SpawnPoint_C|SetChosen%20Animal%20Mesh _array_element (.skeletalmesh (Variables|Runtime|Plushie|GetCurrent%20Animal%20Data)))
    (Default|GameplayManagerFinsihedSetup _array_element)
    (Actor|DestroyActor _array_element))
  ;[0.1316 0.3627 0.5521 0.5] return
  (return))

(fn SetupDataArrays
  (Variables|Runtime|Plushie|SetCurrent%20Spawn%20Iteration 0)
  (Utilities|Array|Shuffle (Variables|CompileTime|Plushie|GetColors%20Array))
  (Utilities|Array|Shuffle (Variables|CompileTime|Plushie|GetRooms%20Array))
  (for _array_element (Variables|CompileTime|Plushie|GetRooms%20Array)
    (Utilities|Map|Add (Variables|Runtime|Plushie|GetRoom%20Type%20to%20Color) _array_element (Utilities|Array|Get(acopy) (Variables|CompileTime|Plushie|GetColors%20Array) (Variables|Runtime|Plushie|GetCurrent%20Spawn%20Iteration)))
    (Math|Integer|IncrementInt (Variables|Runtime|Plushie|GetCurrent%20Spawn%20Iteration)))
  ;[0.1316 0.3627 0.5521 0.5] return
  (return))

(fn SetupRoomColors
  (Utilities|FlowControl|Sequence
    (:then_0
      ;[0.1316 0.3627 0.5521 0.5] Set Hallway Color
      (bind (_material _success) (CallFunction|CreateMaterialforRoomType "NewEnumerator9"))
      (if _success
        (Rendering|Material|SetMaterial (Variables|/Game/HouseProject/House/BP_Class/BP_hallway.BP_hallway_C|GetSM_fridge (Variables|Rooms|GetRoom%20Hallway)) 0 _material)
        (Rendering|Material|SetMaterial (Variables|/Game/HouseProject/House/BP_Class/BP_hallway.BP_hallway_C|GetSM_kitchen_door (Variables|Rooms|GetRoom%20Hallway)) 0 _material)
        (Rendering|Material|SetMaterial (Variables|/Game/HouseProject/House/BP_Class/BP_hallway.BP_hallway_C|GetSM_kitchen_door (Variables|Rooms|GetRoom%20Hallway)) 3 _material)))
    (:then_1
      ;[0.1316 0.3627 0.5521 0.5] Set Kitchen Color
      (bind (_material_2 _success_2) (CallFunction|CreateMaterialforRoomType "NewEnumerator10"))
      (if _success_2
        (Rendering|Material|SetMaterial (Variables|/Game/HouseProject/House/BP_Class/BP_1fl_kitchen.BP_1fl_kitchen_C|GetSM_kitchen_door (Variables|Rooms|GetRoom%20Kitchen)) 0 _material_2)))
    (:then_2
      ;[0.1316 0.3627 0.5521 0.5] Set TV Room Color
      (bind (_material_3 _success_3) (CallFunction|CreateMaterialforRoomType "NewEnumerator11"))
      (if _success_3
        (Rendering|Material|SetMaterial (Variables|/Game/HouseProject/House/BP_Class/BP_1fl_livingroom.BP_1fl_livingroom_C|GetSM_kitchen_door (Variables|Rooms|GetRoom%20TV%20Room)) 0 _material_3)))
    (:then_3
      ;[0.1316 0.3627 0.5521 0.5] Set Garage color
      (bind (_material_4 _success_4) (CallFunction|CreateMaterialforRoomType "NewEnumerator12"))
      (if _success_4
        (Rendering|Material|SetMaterial (Variables|/Script/Engine.StaticMeshActor|GetStaticMeshComponent (Variables|Rooms|GetRoom%20Garage)) 1 _material_4)))
    (:then_4
      ;[0.1316 0.3627 0.5521 0.5] Set Boiler Room Color
      (bind (_material_5 _success_5) (CallFunction|CreateMaterialforRoomType "NewEnumerator13"))
      (if _success_5
        (Rendering|Material|SetMaterial (Variables|/Script/Engine.StaticMeshActor|GetStaticMeshComponent (Variables|Rooms|GetRoom%20Boiler%20Room)) 0 _material_5)))
    (:then_5
      ;[0.1316 0.3627 0.5521 0.5] Set Laundry Color
      (bind (_material_6 _success_6) (CallFunction|CreateMaterialforRoomType "NewEnumerator14"))
      (if _success_6
        (Rendering|Material|SetMaterial (Variables|/Script/Engine.StaticMeshActor|GetStaticMeshComponent (Variables|Rooms|GetRoom%20Laundry)) 0 _material_6)))
    (:then_6
      ;[0.1316 0.3627 0.5521 0.5] Set Small Restroom Color
      (bind (_material_7 _success_7) (CallFunction|CreateMaterialforRoomType "NewEnumerator15"))
      (if _success_7
        (Rendering|Material|SetMaterial (Variables|/Script/Engine.StaticMeshActor|GetStaticMeshComponent (Variables|Rooms|GetRoom%20Small%20Restroom)) 1 _material_7)))
    (:then_7
      ;[0.1316 0.3627 0.5521 0.5] Set Small Restroom Color
      (bind (_material_8 _success_8) (CallFunction|CreateMaterialforRoomType "NewEnumerator16"))
      (if _success_8
        (Rendering|Material|SetMaterial (Variables|/Script/Engine.StaticMeshActor|GetStaticMeshComponent (Variables|Rooms|GetRoom%20Shower%20Room)) 0 _material_8)))
    (:then_8
      ;[0.1316 0.3627 0.5521 0.5] Set Big Bathroom Color
      (bind (_material_9 _success_9) (CallFunction|CreateMaterialforRoomType "NewEnumerator17"))
      (if _success_9
        (Rendering|Material|SetMaterial (Variables|/Game/HouseProject/House/BP_Class/BP_2fl_Bathroom.BP_2fl_Bathroom_C|GetSM_kitchen_door (Variables|Rooms|GetRoom%20Big%20Bathroom)) 0 _material_9)))
    (:then_9
      ;[0.1316 0.3627 0.5521 0.5] Set Zen Room Color
      (bind (_material_10 _success_10) (CallFunction|CreateMaterialforRoomType "NewEnumerator18"))
      (if _success_10
        (Rendering|Material|SetMaterial (Variables|/Game/HouseProject/House/BP_Class/BP_2fl_Greenhouse.BP_2fl_Greenhouse_C|GetSM_kitchen_door (Variables|Rooms|GetRoom%20Zen%20Room)) 0 _material_10)))
    (:then_10
      ;[0.1316 0.3627 0.5521 0.5] Set Reading Room Color
      (bind (_material_11 _success_11) (CallFunction|CreateMaterialforRoomType "NewEnumerator19"))
      (if _success_11
        (Rendering|Material|SetMaterial (Variables|/Game/HouseProject/House/BP_Class/BP_2fl_bedroom2.BP_2fl_bedroom2_C|GetSM_kitchen_door (Variables|Rooms|GetRoom%20Reading%20Room)) 1 _material_11)))
    (:then_11
      ;[0.1316 0.3627 0.5521 0.5] Set Computer Room Color
      (bind (_material_12 _success_12) (CallFunction|CreateMaterialforRoomType "NewEnumerator20"))
      (if _success_12
        (Rendering|Material|SetMaterial (Variables|/Game/HouseProject/House/BP_Class/BP_2fl_Restroom.BP_2fl_Restroom_C|GetSM_kitchen_door (Variables|Rooms|GetRoom%20Computer%20Room)) 0 _material_12)))
    (:then_12
      ;[0.1316 0.3627 0.5521 0.5] Set Bedroom Color
      (bind (_material_13 _success_13) (CallFunction|CreateMaterialforRoomType "NewEnumerator21"))
      (if _success_13
        (Rendering|Material|SetMaterial (Variables|/Game/HouseProject/House/BP_Class/BP_2fl_Bedroom3.BP_2fl_Bedroom3_C|GetSM_kitchen_door (Variables|Rooms|GetRoom%20Bedroom)) 0 _material_13)))))

(fn CreateMaterialforRoomType
  (params (Room%20Type :type E_RoomType%20Enum :default "NewEnumerator9"))
  (bind _room_type_to_color (Variables|Runtime|Plushie|GetRoom%20Type%20to%20Color))
  (bind _enums_to_colors (Variables|CompileTime|Plushie|GetEnums%20to%20Colors))
  (bind _value (Utilities|Map|Find _room_type_to_color Room%20Type))
  (bind (_value_2 _returnvalue) (Utilities|Map|Find _enums_to_colors _value))
  (bind _returnvalue_2 (Rendering|Material|CreateDynamicMaterialInstance "/Game/Gameplay/Materials/MI_RoomPaint.MI_RoomPaint" "Hallway Material" "None" :!class /Script/Engine.KismetMaterialLibrary))
  (if _returnvalue
    (Rendering|Material|SetVectorParameterValue _returnvalue_2 "Room Paint" (Math|Conversions|ToLinearColor(Color) _value_2) :!class /Script/Engine.MaterialInstanceDynamic))
  (return _returnvalue_2 _returnvalue))

(fn SetupChestDataandPlayerSpawn
  (bind _outactors (Actor|GetAllActorsOfClass "/Game/Gameplay/GameplayManager/BP_ChestSpawnPoint.BP_ChestSpawnPoint_C"))
  (Utilities|Array|Shuffle _outactors)
  (bind _returnvalue (Game|SpawnActorfromClass (Variables|CompileTime|Chest|GetChest%20Class) (Math|Transform|MakeTransform (.location (Transformation|GetActorTransform (Utilities|Array|Get(acopy) _outactors))) (.rotation (Transformation|GetActorTransform (Utilities|Array|Get(acopy) _outactors))) "1.000000,1.000000,1.000000") "AlwaysSpawn" "MultiplyWithRoot" 0 (Game|Player|GetPlayerPawn 0)))
  (Variables|Runtime|Chest|SetSpawned%20Chest _returnvalue)
  (bind _asbp_player_character (Utilities|Casting|CastToBP_PlayerCharacter (Game|Player|GetPlayerPawn 0)))
  (Transformation|SetActorLocation _asbp_player_character (Transformation|GetWorldLocation (Variables|/Game/Gameplay/GameplayManager/BP_ChestSpawnPoint.BP_ChestSpawnPoint_C|GetPlayer%20Spawn%20Point (Utilities|Array|Get(acopy) _outactors))) false false)
  (Pawn|SetControlRotation (Game|GetPlayerController 0) (Transformation|GetWorldRotation (Variables|/Game/Gameplay/GameplayManager/BP_ChestSpawnPoint.BP_ChestSpawnPoint_C|GetPlayer%20Spawn%20Point (Utilities|Array|Get(acopy) _outactors))))
  (for _array_element _outactors
    (Actor|DestroyActor _array_element)))

(fn TickTimer
  (bind _output_get (Variables|Timer|SetCurrent%20Time (- (Variables|Timer|GetCurrent%20Time) (Utilities|Time|GetWorldDeltaSeconds))))
  (if (!= (Math|Float|Clamp(Float) _output_get 0.0 (Variables|Timer|GetStart%20Time)) 0.0)
    (Default|CallTimeUpdate (Math|Float|Clamp(Float) _output_get 0.0 (Variables|Timer|GetStart%20Time)))
    (else
      (Utilities|Time|ClearandInvalidateTimerbyHandle (Variables|Timer|GetTimer%20Handle))
      (Default|CallTimerFinished))))

(fn ChooseQuestionsandGenerateAnswers)

(fn FindCorrectAnswers
  (bind _questions_data (Variables|Default|GetQuestions%20Data))
  (bind _output (Utilities|Array|Get(acopy) _questions_data))
  (Utilities|FlowControl|Sequence
    (:then_0
      ;[0.1316 0.3627 0.5521 0.5] Find total sum of all Animals
      (for _array_element (Variables|Default|GetQuestions%20Data)
        (LocalVariables|SetTotalPrice (+ (.price (.gameplaydata _array_element)) (LocalVariables|GetTotalPrice))))
      (Utilities|Map|Add (Variables|Default|GetCorrectAnswers) "NewEnumerator0" (Utilities|String|ToString(Integer) (LocalVariables|GetTotalPrice))))
    (:then_1
      ;[0.1316 0.3627 0.5521 0.5] Find Highest/Lowest price Animal
      (LocalVariables|SetCurrent%20HIghest%20Price (.price (.gameplaydata _output)))
      (LocalVariables|SetCurrent%20Lowest%20Price (.price (.gameplaydata _output)))
      (for _array_element_2 (Variables|Default|GetQuestions%20Data)
        (Utilities|FlowControl|Sequence
          (:then_0
            (if (> (.price (.gameplaydata _array_element_2)) (LocalVariables|GetCurrent%20HIghest%20Price))
              (LocalVariables|SetCurrent%20HIghest%20Price (.price (.gameplaydata _array_element_2)))))
          (:then_1
            (if (< (.price (.gameplaydata _array_element_2)) (LocalVariables|GetCurrent%20Lowest%20Price))
              (LocalVariables|SetCurrent%20Lowest%20Price (.price (.gameplaydata _array_element_2)))))))
      (Utilities|Map|Add (Variables|Default|GetCorrectAnswers) "NewEnumerator1" (Utilities|String|ToString(Integer) (LocalVariables|GetCurrent%20HIghest%20Price)))
      (Utilities|Map|Add (Variables|Default|GetCorrectAnswers) "NewEnumerator2" (Utilities|String|ToString(Integer) (LocalVariables|GetCurrent%20Lowest%20Price))))
    (:then_2
      ;[0.1316 0.3627 0.5521 0.5] Find Room type for Highest/Lowest price animal, Room color for Highest/Lowest price animal, Animal type for Highest/Lowest price
      (for _array_element_3 (Variables|Default|GetQuestions%20Data)
        (Utilities|FlowControl|Sequence
          (:then_0
            (if (== (.price (.gameplaydata _array_element_3)) (LocalVariables|GetCurrent%20HIghest%20Price))
              (LocalVariables|SetCurrent%20Room%20Type%20Highest%20Price (.roomtype (.spawndata _array_element_3)))
              (LocalVariables|SetCurrent%20Room%20Color%20Highest%20Price (.roomcolor (.gameplaydata _array_element_3)))
              (LocalVariables|SetCurrent%20Animal%20With%20Highest%20Price (.animal (.gameplaydata _array_element_3)))))
          (:then_1
            (if (== (.price (.gameplaydata _array_element_3)) (LocalVariables|GetCurrent%20Lowest%20Price))
              (LocalVariables|SetCurrent%20Room%20Type%20Lowest%20Price (.roomtype (.spawndata _array_element_3)))
              (LocalVariables|SetCurrent%20Room%20Color%20Lowest%20Price (.roomcolor (.gameplaydata _array_element_3)))
              (LocalVariables|SetCurrent%20Animal%20With%20Lowest%20Price (.animal (.gameplaydata _array_element_3)))))))
      (Utilities|Map|Add (Variables|Default|GetCorrectAnswers) "NewEnumerator3" (Utilities|String|EnumtoString (LocalVariables|GetCurrent%20Room%20Type%20Highest%20Price)))
      (Utilities|Map|Add (Variables|Default|GetCorrectAnswers) "NewEnumerator4" (Utilities|String|EnumtoString (LocalVariables|GetCurrent%20Room%20Type%20Lowest%20Price)))
      (Utilities|Map|Add (Variables|Default|GetCorrectAnswers) "NewEnumerator5" (Utilities|String|EnumtoString (LocalVariables|GetCurrent%20Room%20Color%20Highest%20Price)))
      (Utilities|Map|Add (Variables|Default|GetCorrectAnswers) "NewEnumerator6" (Utilities|String|EnumtoString (LocalVariables|GetCurrent%20Room%20Color%20Lowest%20Price)))
      (Utilities|Map|Add (Variables|Default|GetCorrectAnswers) "NewEnumerator11" (Utilities|String|EnumtoString (LocalVariables|GetCurrent%20Animal%20With%20Highest%20Price)))
      (Utilities|Map|Add (Variables|Default|GetCorrectAnswers) "NewEnumerator12" (Utilities|String|EnumtoString (LocalVariables|GetCurrent%20Animal%20With%20Lowest%20Price))))
    (:then_3
      ;[0.1316 0.3627 0.5521 0.5] Calculate Carnivores, Herbivores, Flying and Swimming animals
      (for _array_element_4 (Variables|Default|GetQuestions%20Data)
        (Utilities|FlowControl|Sequence
          (:then_0
            (if (.iscarnivore (.gameplaydata _array_element_4))
              (Math|Integer|IncrementInt (LocalVariables|GetNumber%20of%20Carnivores))))
          (:then_1
            (if (.isherbivore (.gameplaydata _array_element_4))
              (Math|Integer|IncrementInt (LocalVariables|GetNumber%20of%20Herbivores))))
          (:then_2
            (if (.isflying (.gameplaydata _array_element_4))
              (Math|Integer|IncrementInt (LocalVariables|GetNumber%20of%20Flying))))
          (:then_3
            (if (.isswimming (.gameplaydata _array_element_4))
              (Math|Integer|IncrementInt (LocalVariables|GetNumber%20of%20Swimming))))))
      (Utilities|Map|Add (Variables|Default|GetCorrectAnswers) "NewEnumerator7" (Utilities|String|ToString(Integer) (LocalVariables|GetNumber%20of%20Carnivores)))
      (Utilities|Map|Add (Variables|Default|GetCorrectAnswers) "NewEnumerator8" (Utilities|String|ToString(Integer) (LocalVariables|GetNumber%20of%20Herbivores)))
      (Utilities|Map|Add (Variables|Default|GetCorrectAnswers) "NewEnumerator9" (Utilities|String|ToString(Integer) (LocalVariables|GetNumber%20of%20Flying)))
      (Utilities|Map|Add (Variables|Default|GetCorrectAnswers) "NewEnumerator10" (Utilities|String|ToString(Integer) (LocalVariables|GetNumber%20of%20Swimming))))
    (:then_4
      (return))))

(fn ShowTutorialifNeeded
  (bind _returnvalue (Game|GetPlayerController 0))
  (bind _asbp_game_instance (Utilities|Casting|CastToBP_GameInstance (Game|GetGameInstance)))
  (if (Variables|/Game/Gameplay/Core/BP_GameInstance.BP_GameInstance_C|GetShow%20Tutorial _asbp_game_instance)
    (Variables|/Game/Gameplay/Core/BP_GameInstance.BP_GameInstance_C|SetShow%20Tutorial _asbp_game_instance false)
    (bind _returnvalue_2 (UserInterface|CreateWidget "/Game/UI/WBP_Tutorial.WBP_Tutorial_C"))
    (UserInterface|Viewport|AddtoViewport _returnvalue_2 0)
    (Input|SetInputModeGameandUI _returnvalue _returnvalue_2 "LockInFullscreen" false true)
    (Variables|/Script/Engine.PlayerController|SetbShowMouseCursor _returnvalue true)
    (Game|SetGamePaused true)
    (Variables|Default|SetGame%20State "NewEnumerator2")
    (else
      (Variables|Default|SetGame%20State "NewEnumerator1")))
  (return))