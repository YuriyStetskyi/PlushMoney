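; BP_SpawnPoint is a placeable marker that spawns a BP_Plushie into the level.
; The construction script caches the Sphere component's world location and rotation, plus the room type, as spawn data.
; When GameplayManagerFinsihedSetup fires, it spawns the plushie at that transform regardless of collision, then applies the chosen animal mesh and passes on gameplay and spawn data.
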(event Custom|Gameplay%20Manager%20Finsihed%20Setup
  (bind _plushie_spawn_data (Variables|Data|GetPlushie%20Spawn%20Data))
  (bind _returnvalue (Game|SpawnActorfromClass "/Game/Gameplay/Actors/BP_Plushie.BP_Plushie_C" (Math|Transform|MakeTransform (.location _plushie_spawn_data) (.rotation _plushie_spawn_data) "1.000000,1.000000,1.000000") "AlwaysSpawn" "MultiplyWithRoot" 0 (Game|Player|GetPlayerPawn 0)))
  (bind _output_get (Variables|Runtime|SetSpawned%20Plushie _returnvalue))
  (Components|SkeletalMesh|SetSkeletalMeshAsset (Variables|/Game/Gameplay/Actors/BP_Plushie.BP_Plushie_C|GetSkeletalMesh _output_get) (Variables|Runtime|GetChosen%20Animal%20Mesh))
  (Variables|/Game/Gameplay/Actors/BP_Plushie.BP_Plushie_C|SetGameplay%20Data (Variables|Runtime|GetSpawned%20Plushie) (Variables|Data|GetPlushie%20Gameplay%20Data))
  (Variables|/Game/Gameplay/Actors/BP_Plushie.BP_Plushie_C|SetSpawn%20Data (Variables|Runtime|GetSpawned%20Plushie) (Variables|Data|GetPlushie%20Spawn%20Data)))

(event EventBeginPlay)

(event Collision|EventActorBeginOverlap
  (params (OtherActor :type Actor%20Object%20Reference)))

(event EventTick
  (params (DeltaSeconds :type Float%20%28single-precision%29)))

(fn ConstructionScript
  (Variables|Data|SetPlushie%20Spawn%20Data (Utilities|Struct|MakeF_PlushieSpawnData (Transformation|GetWorldLocation (Variables|Default|GetSphere)) (Transformation|GetWorldRotation (Variables|Default|GetSphere)) (Variables|Data|GetPlushie%20Room%20Type))))