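; BP_ScoreChest is the drop-off actor where plushies are turned in.
; Its box overlap detects Plushie-tagged actors, broadcasts the plushie-turned-in event with their gameplay and spawn data, then destroys them.
; The chest also binds to that event on BeginPlay, responding with a floating popup widget showing the animal name and price, plus a cash register sound.
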(event OnComponentBeginOverlap(Box)
  (params (OverlappedComponent :type Primitive%20Component%20Object%20Reference) (OtherActor :type Actor%20Object%20Reference) (OtherComp :type Primitive%20Component%20Object%20Reference) (OtherBodyIndex :type Integer) (bFromSweep :type Boolean) (SweepResult :type Hit%20Result%20Structure%20%28by%20ref%29))
  (if (Actor|ActorHasTag OtherActor "Plushie")
    (bind _asbp_plushie (Utilities|Casting|CastToBP_Plushie OtherActor))
    (Default|CallPlushieTurnedin (Variables|/Game/Gameplay/Actors/BP_Plushie.BP_Plushie_C|GetGameplay%20Data _asbp_plushie) (Variables|/Game/Gameplay/Actors/BP_Plushie.BP_Plushie_C|GetSpawn%20Data _asbp_plushie))
    (Actor|DestroyActor _asbp_plushie)))

(event Custom|Display%20Price%20Widget
  (params (Plushie%20Gameplay%20Data :type F%20Plushie%20Manager%20Data%20Structure) (Plushie%20Spawn%20Data :type F%20Plushie%20Spawn%20Data%20Structure))
  (bind _returnvalue (UserInterface|CreateWidget "/Game/UI/WBP_PopupPlushieCollected.WBP_PopupPlushieCollected_C" 0 (.price Plushie%20Gameplay%20Data) (Utilities|Text|ToText(String) (Utilities|String|EnumtoString (.animal Plushie%20Gameplay%20Data)))))
  (UserInterface|Viewport|AddtoViewport _returnvalue 0)
  (Default|StartTextFloat _returnvalue)
  (Audio|PlaySound2D "/Game/Assets/Sounds/cash_register.cash_register" 1.0 0.92 0.0 0 0))

(event EventBeginPlay
  (EventDispatchers|BindEventtoPlushieTurnedin (delegate Custom|Display%20Price%20Widget)))

(event Collision|EventActorBeginOverlap
  (params (OtherActor :type Actor%20Object%20Reference)))

(event EventTick
  (params (DeltaSeconds :type Float%20%28single-precision%29)))

(fn ConstructionScript)