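; BP_Plushie is a plushie actor that the player character can hold and release.
; StartHolding and StopHolding respond only to BP_PlayerCharacter, switching gravity and physics simulation on the CollisionBox off while held and back on when released.
; While the box simulates physics, Tick clamps each axis of its linear velocity to plus or minus MaxPhysicsVelocity.
; The Interact event is empty.
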(event EventBeginPlay)

(event Collision|EventActorBeginOverlap
  (params (OtherActor :type Actor%20Object%20Reference)))

(event EventTick
  (params (DeltaSeconds :type Float%20%28single-precision%29))
  (bind _collision_box (Variables|Default|GetCollision%20Box))
  (bind _max_physics_velocity (Variables|Default|GetMax%20Physics%20Velocity))
  (bind _returnvalue (* _max_physics_velocity -1.0))
  (if (Physics|IsSimulatingPhysics _collision_box "None")
    (bind _returnvalue_2 (Physics|GetPhysicsLinearVelocity _collision_box "None"))
    (Physics|SetPhysicsLinearVelocity _collision_box (Math|Vector|MakeVector (Math|Float|Clamp(Float) (.x _returnvalue_2) _returnvalue _max_physics_velocity) (Math|Float|Clamp(Float) (.y _returnvalue_2) _returnvalue _max_physics_velocity) (Math|Float|Clamp(Float) (.z _returnvalue_2) _returnvalue _max_physics_velocity)) false "None")))

(event EventInteract
  (params (Interacted%20Actor :type Actor%20Object%20Reference)))

(event EventStartHolding
  (params (Holding%20Actor :type Actor%20Object%20Reference))
  (bind _collision_box (Variables|Default|GetCollision%20Box))
  (Utilities|Casting|CastToBP_PlayerCharacter Holding%20Actor)
  (Physics|SetEnableGravity _collision_box false)
  (Physics|SetSimulatePhysics _collision_box false))

(event EventStopHolding
  (params (Holding%20Actor :type Actor%20Object%20Reference))
  (bind _collision_box (Variables|Default|GetCollision%20Box))
  (Utilities|Casting|CastToBP_PlayerCharacter Holding%20Actor)
  (Physics|SetEnableGravity _collision_box true)
  (Physics|SetSimulatePhysics _collision_box true))

(fn ConstructionScript)