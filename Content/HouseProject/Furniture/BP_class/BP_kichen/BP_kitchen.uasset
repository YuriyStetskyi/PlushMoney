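; Kitchen furniture actor that lets the player cycle the finish of the kitchen door and fridge meshes.
; Entering or leaving the Box trigger enables or disables the actor's input for player 0 and toggles two text render labels.
; Each left mouse click steps a looping MultiGate, starting at its second output, to apply one of six materials to slot 1 of both meshes.
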(event OnComponentBeginOverlap(Box)
  (params (OverlappedComponent :type Primitive%20Component%20Object%20Reference) (OtherActor :type Actor%20Object%20Reference) (OtherComp :type Primitive%20Component%20Object%20Reference) (OtherBodyIndex :type Integer) (bFromSweep :type Boolean) (SweepResult :type Hit%20Result%20Structure%20%28by%20ref%29))
  (Input|EnableInput (Game|GetPlayerController 0))
  (Rendering|ToggleVisibility (Variables|Default|GetTextRender) false))

(event OnComponentEndOverlap(Box)
  (params (OverlappedComponent :type Primitive%20Component%20Object%20Reference) (OtherActor :type Actor%20Object%20Reference) (OtherComp :type Primitive%20Component%20Object%20Reference) (OtherBodyIndex :type Integer))
  (Input|DisableInput (Game|GetPlayerController 0))
  (Rendering|ToggleVisibility (Variables|Default|GetTextRender) false))

(event Input|MouseEvents|LeftMouseButton
  (params (Key :type Key%20Structure :default "None"))
  (:Pressed
    (Utilities|FlowControl|MultiGate false true 1
      (:Out%200
        (Rendering|Material|SetMaterial (Variables|Default|GetSM_kitchen_door) 1 "/Game/HouseProject/Furniture/Kitchen/Material/Material_BP/M_kichen1.M_kichen1")
        (Rendering|Material|SetMaterial (Variables|Default|GetSM_fridge) 1 "/Game/HouseProject/Furniture/Kitchen/Material/Material_BP/M_kichen1.M_kichen1"))
      (:Out%201
        (Rendering|Material|SetMaterial (Variables|Default|GetSM_kitchen_door) 1 "/Game/HouseProject/Furniture/Kitchen/Material/M_kichen02.M_kichen02")
        (Rendering|Material|SetMaterial (Variables|Default|GetSM_fridge) 1 "/Game/HouseProject/Furniture/Kitchen/Material/M_kichen02.M_kichen02"))
      (:Out%202
        (Rendering|Material|SetMaterial (Variables|Default|GetSM_kitchen_door) 1 "/Game/HouseProject/Furniture/Kitchen/Material/Material_BP/M_kichen2.M_kichen2")
        (Rendering|Material|SetMaterial (Variables|Default|GetSM_fridge) 1 "/Game/HouseProject/Furniture/Kitchen/Material/Material_BP/M_kichen2.M_kichen2"))
      (:Out%203
        (Rendering|Material|SetMaterial (Variables|Default|GetSM_kitchen_door) 1 "/Game/HouseProject/Furniture/Kitchen/Material/Material_BP/M_kichen3.M_kichen3")
        (Rendering|Material|SetMaterial (Variables|Default|GetSM_fridge) 1 "/Game/HouseProject/Furniture/Kitchen/Material/Material_BP/M_kichen3.M_kichen3"))
      (:Out%204
        (Rendering|Material|SetMaterial (Variables|Default|GetSM_kitchen_door) 1 "/Game/HouseProject/Furniture/Kitchen/Material/Material_BP/M_kichen4.M_kichen4")
        (Rendering|Material|SetMaterial (Variables|Default|GetSM_fridge) 1 "/Game/HouseProject/Furniture/Kitchen/Material/Material_BP/M_kichen4.M_kichen4"))
      (:Out%205
        (Rendering|Material|SetMaterial (Variables|Default|GetSM_kitchen_door) 1 "/Game/HouseProject/Furniture/Kitchen/Material/Material_BP/M_kichen6.M_kichen6")
        (Rendering|Material|SetMaterial (Variables|Default|GetSM_fridge) 1 "/Game/HouseProject/Furniture/Kitchen/Material/Material_BP/M_kichen6.M_kichen6")))))

(fn ConstructionScript)