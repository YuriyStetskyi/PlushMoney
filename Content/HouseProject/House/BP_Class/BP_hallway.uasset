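; Hallway Blueprint in the house project that lets the player cycle wall finishes on nearby meshes.
; A Box trigger enables player input on overlap and disables it on exit, toggling two text prompts both times.
; While input is enabled, left click advances a looping MultiGate, starting at its second output, through ten wallpaper and color presets.
; Each preset sets materials on two slots of SMKitchenDoor and one slot of SMFridge.
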(event OnComponentBeginOverlap(Box)
  (params (OverlappedComponent :type Primitive%20Component%20Object%20Reference) (OtherActor :type Actor%20Object%20Reference) (OtherComp :type Primitive%20Component%20Object%20Reference) (OtherBodyIndex :type Integer) (bFromSweep :type Boolean) (SweepResult :type Hit%20Result%20Structure%20%28by%20ref%29))
  (Input|EnableInput (Game|GetPlayerController 0))
  (Rendering|ToggleVisibility (Variables|Default|GetTextRender) false))

(event OnComponentEndOverlap(Box)
  (params (OverlappedComponent :type Primitive%20Component%20Object%20Reference) (OtherActor :type Actor%20Object%20Reference) (OtherComp :type Primitive%20Component%20Object%20Reference) (OtherBodyIndex :type Integer))
  (Input|DisableInput (Game|GetPlayerController 0))
  (Rendering|ToggleVisibility (Variables|Default|GetTextRender) false))

(event Input|MouseEvents|LeftMouseButton
  (params (Key :type Key%20Structure :default "None"))
  (bind _sm_kitchen_door (Variables|Default|GetSM_kitchen_door))
  (bind _sm_kitchen_door_2 (Variables|Default|GetSM_kitchen_door))
  (bind _sm_fridge (Variables|Default|GetSM_fridge))
  (:Pressed
    (Utilities|FlowControl|MultiGate false true 1
      (:Out%200
        (Rendering|Material|SetMaterial _sm_kitchen_door 3 "/Game/HouseProject/House/Materials/wallpaper/M_wallpaper_020.M_wallpaper_020")
        (Rendering|Material|SetMaterial _sm_kitchen_door_2 0 "/Game/HouseProject/House/Materials/wallpaper/M_wallpaper_020.M_wallpaper_020")
        (Rendering|Material|SetMaterial (Variables|Default|GetSM_fridge) 0 "/Game/HouseProject/House/Materials/wallpaper/M_wallpaper_021.M_wallpaper_021"))
      (:Out%201
        (Rendering|Material|SetMaterial _sm_kitchen_door 3 "/Game/HouseProject/House/Materials/wallpaper/M_wallpaper_018_2.M_wallpaper_018_2")
        (Rendering|Material|SetMaterial _sm_kitchen_door_2 0 "/Game/HouseProject/House/Materials/wallpaper/M_wallpaper_018_2.M_wallpaper_018_2")
        (Rendering|Material|SetMaterial (Variables|Default|GetSM_fridge) 0 "/Game/HouseProject/House/Materials/wallpaper/M_wallpaper_018_2.M_wallpaper_018_2"))
      (:Out%202
        (Rendering|Material|SetMaterial _sm_kitchen_door 3 "/Game/HouseProject/House/Materials/wallpaper/M_wallpaper_013_2.M_wallpaper_013_2")
        (Rendering|Material|SetMaterial _sm_kitchen_door_2 0 "/Game/HouseProject/House/Materials/wallpaper/M_wallpaper_013_2.M_wallpaper_013_2")
        (Rendering|Material|SetMaterial (Variables|Default|GetSM_fridge) 0 "/Game/HouseProject/House/Materials/wallpaper/M_wallpaper_013_2.M_wallpaper_013_2"))
      (:Out%203
        (Rendering|Material|SetMaterial _sm_kitchen_door 3 "/Game/HouseProject/House/Materials/wallpaper/M_wallpaper_019_2.M_wallpaper_019_2")
        (Rendering|Material|SetMaterial _sm_kitchen_door_2 0 "/Game/HouseProject/House/Materials/wallpaper/M_wallpaper_019_2.M_wallpaper_019_2")
        (Rendering|Material|SetMaterial (Variables|Default|GetSM_fridge) 0 "/Game/HouseProject/House/Materials/wallpaper/M_wallpaper_019_2.M_wallpaper_019_2"))
      (:Out%204
        (Rendering|Material|SetMaterial _sm_kitchen_door 3 "/Game/HouseProject/House/Materials/wallpaper/M_wallpaper_012.M_wallpaper_012")
        (Rendering|Material|SetMaterial _sm_kitchen_door_2 0 "/Game/HouseProject/House/Materials/wallpaper/M_wallpaper_012.M_wallpaper_012")
        (Rendering|Material|SetMaterial (Variables|Default|GetSM_fridge) 0 "/Game/HouseProject/House/Materials/wallpaper/M_wallpaper_012.M_wallpaper_012"))
      (:Out%205
        (Rendering|Material|SetMaterial _sm_kitchen_door 3 "/Game/HouseProject/House/Materials/wallpaper/M_wallpaper_018_3.M_wallpaper_018_3")
        (Rendering|Material|SetMaterial _sm_kitchen_door_2 0 "/Game/HouseProject/House/Materials/wallpaper/M_wallpaper_018_3.M_wallpaper_018_3")
        (Rendering|Material|SetMaterial _sm_fridge 0 "/Game/HouseProject/House/Materials/wallpaper/M_wallpaper_018_3.M_wallpaper_018_3"))
      (:Out%206
        (Rendering|Material|SetMaterial _sm_kitchen_door 3 "/Game/HouseProject/House/Materials/wallpaper/M_wallpaper_054_2.M_wallpaper_054_2")
        (Rendering|Material|SetMaterial _sm_kitchen_door_2 0 "/Game/HouseProject/House/Materials/wallpaper/M_wallpaper_054_2.M_wallpaper_054_2")
        (Rendering|Material|SetMaterial _sm_fridge 0 "/Game/HouseProject/House/Materials/wallpaper/M_wallpaper_054_2.M_wallpaper_054_2"))
      (:Out%207
        (Rendering|Material|SetMaterial _sm_kitchen_door 3 "/Game/HouseProject/House/Materials/Color/M_color3.M_color3")
        (Rendering|Material|SetMaterial _sm_kitchen_door_2 0 "/Game/HouseProject/House/Materials/Color/M_color3.M_color3")
        (Rendering|Material|SetMaterial _sm_fridge 0 "/Game/HouseProject/House/Materials/Color/M_color3.M_color3"))
      (:Out%208
        (Rendering|Material|SetMaterial _sm_kitchen_door 3 "/Game/HouseProject/House/Materials/Color/M_color2.M_color2")
        (Rendering|Material|SetMaterial _sm_kitchen_door_2 0 "/Game/HouseProject/House/Materials/Color/M_color2.M_color2")
        (Rendering|Material|SetMaterial _sm_fridge 0 "/Game/HouseProject/House/Materials/Color/M_color2.M_color2"))
      (:Out%209
        (Rendering|Material|SetMaterial _sm_kitchen_door 3 "/Game/HouseProject/House/Materials/Color/M_color4.M_color4")
        (Rendering|Material|SetMaterial _sm_kitchen_door_2 0 "/Game/HouseProject/House/Materials/Color/M_color4.M_color4")
        (Rendering|Material|SetMaterial _sm_fridge 0 "/Game/HouseProject/House/Materials/Color/M_color4.M_color4")))))

(fn ConstructionScript)