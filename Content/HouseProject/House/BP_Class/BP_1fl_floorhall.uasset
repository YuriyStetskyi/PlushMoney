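; Interactive first-floor hall prop, apparently the floor, that lets the player cycle its surface finish among tile and wooden-tile materials.
; Overlapping the Box enables player input on the actor and leaving disables it, with both events toggling the two TextRender components' visibility.
; Each right mouse press advances a looping, sequential MultiGate, starting at its second output, that swaps the first material slot of the mesh component named SMKitchenDoor.
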(event OnComponentBeginOverlap(Box)
  (params (OverlappedComponent :type Primitive%20Component%20Object%20Reference) (OtherActor :type Actor%20Object%20Reference) (OtherComp :type Primitive%20Component%20Object%20Reference) (OtherBodyIndex :type Integer) (bFromSweep :type Boolean) (SweepResult :type Hit%20Result%20Structure%20%28by%20ref%29))
  (Input|EnableInput (Game|GetPlayerController 0))
  (Rendering|ToggleVisibility (Variables|Default|GetTextRender) false))

(event OnComponentEndOverlap(Box)
  (params (OverlappedComponent :type Primitive%20Component%20Object%20Reference) (OtherActor :type Actor%20Object%20Reference) (OtherComp :type Primitive%20Component%20Object%20Reference) (OtherBodyIndex :type Integer))
  (Input|DisableInput (Game|GetPlayerController 0))
  (Rendering|ToggleVisibility (Variables|Default|GetTextRender) false))

(event Input|MouseEvents|LeftMouseButton
  (params (Key :type Key%20Structure :default "None")))

(event Input|MouseEvents|RightMouseButton
  (params (Key :type Key%20Structure :default "None"))
  (bind _sm_kitchen_door (Variables|Default|GetSM_kitchen_door))
  (bind _sm_kitchen_door_2 (Variables|Default|GetSM_kitchen_door))
  (bind _sm_kitchen_door_3 (Variables|Default|GetSM_kitchen_door))
  (:Pressed
    (Utilities|FlowControl|MultiGate false true 1
      (:Out%200
        (Rendering|Material|SetMaterial _sm_kitchen_door 0 "/Game/HouseProject/House/Materials/tile/house/M_title_020.M_title_020"))
      (:Out%201
        (Rendering|Material|SetMaterial _sm_kitchen_door 0 "/Game/HouseProject/House/Materials/tile/house/M_title_01_2.M_title_01_2"))
      (:Out%202
        (Rendering|Material|SetMaterial _sm_kitchen_door_2 0 "/Game/HouseProject/House/Materials/tile/house/M_title_009_2.M_title_009_2"))
      (:Out%203
        (Rendering|Material|SetMaterial _sm_kitchen_door_3 0 "/Game/HouseProject/House/Materials/tile/house/M_title_012_2.M_title_012_2"))
      (:Out%204
        (Rendering|Material|SetMaterial _sm_kitchen_door_3 0 "/Game/HouseProject/House/Materials/tile/house/M_title_03_2.M_title_03_2"))
      (:Out%205
        (Rendering|Material|SetMaterial _sm_kitchen_door_3 0 "/Game/HouseProject/House/Materials/Wooden_Tiles/M_Wooden_Tiles_005.M_Wooden_Tiles_005"))
      (:Out%206
        (Rendering|Material|SetMaterial _sm_kitchen_door_2 0 "/Game/HouseProject/House/Materials/Wooden_Tiles/M_Wooden_Tiles_001_2.M_Wooden_Tiles_001_2"))
      (:Out%207
        (Rendering|Material|SetMaterial _sm_kitchen_door_2 0 "/Game/HouseProject/House/Materials/Wooden_Tiles/M_Wooden_Tiles_002_2.M_Wooden_Tiles_002_2"))
      (:Out%208
        (Rendering|Material|SetMaterial _sm_kitchen_door_2 0 "/Game/HouseProject/House/Materials/Wooden_Tiles/M_Wooden_Tiles_003_2.M_Wooden_Tiles_003_2"))
      (:Out%209
        (Rendering|Material|SetMaterial _sm_kitchen_door_2 0 "/Game/HouseProject/House/Materials/Wooden_Tiles/M_Wooden_Tiles_006_2.M_Wooden_Tiles_006_2"))
      (:Out%2010
        (Rendering|Material|SetMaterial _sm_kitchen_door_2 0 "/Game/HouseProject/House/Materials/Wooden_Tiles/M_Wooden_Tiles_004_2.M_Wooden_Tiles_004_2")))))

(fn ConstructionScript)