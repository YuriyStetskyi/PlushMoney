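; Second-floor bathroom Blueprint for the house project that lets the player cycle materials on a mesh component (SMKitchenDoor).
; Entering the Box trigger enables player input and leaving disables it, with both events toggling the visibility of two text renders.
; While input is enabled, left mouse clicks step a looping MultiGate through seven M_title materials, applying each to both material slots.
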(event OnComponentBeginOverlap(Box)
  (params (OverlappedComponent :type Primitive%20Component%20Object%20Reference) (OtherActor :type Actor%20Object%20Reference) (OtherComp :type Primitive%20Component%20Object%20Reference) (OtherBodyIndex :type Integer) (bFromSweep :type Boolean) (SweepResult :type Hit%20Result%20Structure%20%28by%20ref%29))
  (Input|EnableInput (Game|GetPlayerController 0))
  (Rendering|ToggleVisibility (Variables|Default|GetTextRender) false))

(event OnComponentEndOverlap(Box)
  (params (OverlappedComponent :type Primitive%20Component%20Object%20Reference) (OtherActor :type Actor%20Object%20Reference) (OtherComp :type Primitive%20Component%20Object%20Reference) (OtherBodyIndex :type Integer))
  (Input|DisableInput (Game|GetPlayerController 0))
  (Rendering|ToggleVisibility (Variables|Default|GetTextRender) false))

(event Input|MouseEvents|LeftMouseButton
  (params (Key :type Key%20Structure :default "None"))
  (bind _sm_kitchen_door (Variables|Default|GetSM_kitchen_door))
  (bind _sm_kitchen_door_2 (Variables|Default|GetSM_kitchen_door))
  (:Pressed
    (Utilities|FlowControl|MultiGate false true 1
      (:Out%200
        (Rendering|Material|SetMaterial _sm_kitchen_door_2 0 "/Game/HouseProject/House/Materials/tile/Bathroom/M_title_007_2.M_title_007_2")
        (Rendering|Material|SetMaterial _sm_kitchen_door 1 "/Game/HouseProject/House/Materials/tile/Bathroom/M_title_007_2.M_title_007_2"))
      (:Out%201
        (Rendering|Material|SetMaterial _sm_kitchen_door_2 0 "/Game/HouseProject/House/Materials/tile/Bathroom/M_title_008_2.M_title_008_2")
        (Rendering|Material|SetMaterial _sm_kitchen_door 1 "/Game/HouseProject/House/Materials/tile/Bathroom/M_title_008_2.M_title_008_2"))
      (:Out%202
        (Rendering|Material|SetMaterial _sm_kitchen_door_2 0 "/Game/HouseProject/House/Materials/tile/Bathroom/M_title_009.M_title_009")
        (Rendering|Material|SetMaterial _sm_kitchen_door 1 "/Game/HouseProject/House/Materials/tile/Bathroom/M_title_009.M_title_009"))
      (:Out%203
        (Rendering|Material|SetMaterial _sm_kitchen_door_2 0 "/Game/HouseProject/House/Materials/tile/Bathroom/M_title_010.M_title_010")
        (Rendering|Material|SetMaterial _sm_kitchen_door 1 "/Game/HouseProject/House/Materials/tile/Bathroom/M_title_010.M_title_010"))
      (:Out%204
        (Rendering|Material|SetMaterial _sm_kitchen_door_2 0 "/Game/HouseProject/House/Materials/tile/Bathroom/M_title_011.M_title_011")
        (Rendering|Material|SetMaterial _sm_kitchen_door 1 "/Game/HouseProject/House/Materials/tile/Bathroom/M_title_011.M_title_011"))
      (:Out%205
        (Rendering|Material|SetMaterial _sm_kitchen_door_2 0 "/Game/HouseProject/House/Materials/tile/Bathroom/M_title_012.M_title_012")
        (Rendering|Material|SetMaterial _sm_kitchen_door 1 "/Game/HouseProject/House/Materials/tile/Bathroom/M_title_012.M_title_012"))
      (:Out%206
        (Rendering|Material|SetMaterial _sm_kitchen_door_2 0 "/Game/HouseProject/House/Materials/tile/Bathroom/M_title_014.M_title_014")
        (Rendering|Material|SetMaterial _sm_kitchen_door 1 "/Game/HouseProject/House/Materials/tile/Bathroom/M_title_014.M_title_014")))))

(fn ConstructionScript)