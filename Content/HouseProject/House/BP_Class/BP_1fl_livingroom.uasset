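; First-floor living room actor that lets the player cycle the material on the SMKitchenDoor mesh, mostly through wallpapers and colors.
; Entering the Box trigger enables player input and leaving disables it, with both events toggling the visibility of two text renders.
; Each left click advances a looping, sequential MultiGate that sets the next hard-coded material on slot 0, starting from the second entry.
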(event OnComponentBeginOverlap(Box)
  (params (OverlappedComponent :type Primitive%20Component%20Object%20Reference) (OtherActor :type Actor%20Object%20Reference) (OtherComp :type Primitive%20Component%20Object%20Reference) (OtherBodyIndex :type Integer) (bFromSweep :type Boolean) (SweepResult :type Hit%20Result%20Structure%20%28by%20ref%29))
  (Input|EnableInput (Game|GetPlayerController 0))
  (Rendering|ToggleVisibility (Variables|Default|GetTextRender) false))

(event OnComponentEndOverlap(Box)
  (params (OverlappedComponent :type Primitive%20Component%20Object%20Reference) (OtherActor :type Actor%20Object%20Reference) (OtherComp :type Primitive%20Component%20Object%20Reference) (OtherBodyIndex :type Integer))
  (Input|DisableInput (Game|GetPlayerController 0))
  (Rendering|ToggleVisibility (Variables|Default|GetTextRender) false))

(event Input|MouseEvents|LeftMouseButton
  (params (Key :type Key%20Structure :default "None"))
  (bind _sm_kitchen_door (Variables|Default|GetSM_kitchen_door))
  (bind _sm_kitchen_door_2 (Variables|Default|GetSM_kitchen_door))
  (:Pressed
    (Utilities|FlowControl|MultiGate false true 1
      (:Out%200
        (Rendering|Material|SetMaterial _sm_kitchen_door 0 "/Game/HouseProject/House/Materials/wallpaper/M_wallpaper_055.M_wallpaper_055"))
      (:Out%201
        (Rendering|Material|SetMaterial _sm_kitchen_door 0 "/Game/HouseProject/House/Materials/wallpaper/M_wallpaper_018.M_wallpaper_018"))
      (:Out%202
        (Rendering|Material|SetMaterial (Variables|Default|GetSM_kitchen_door) 0 "/Game/HouseProject/House/Materials/wallpaper/M_wallpaper_013.M_wallpaper_013"))
      (:Out%203
        (Rendering|Material|SetMaterial _sm_kitchen_door_2 0 "/Game/HouseProject/House/Materials/wallpaper/M_wallpaper_019.M_wallpaper_019"))
      (:Out%204
        (Rendering|Material|SetMaterial _sm_kitchen_door_2 0 "/Game/HouseProject/House/Materials/wallpaper/M_wallpaper_012.M_wallpaper_012"))
      (:Out%205
        (Rendering|Material|SetMaterial _sm_kitchen_door_2 0 "/Game/HouseProject/House/Materials/wallpaper/M_wallpaper_054.M_wallpaper_054"))
      (:Out%206
        (Rendering|Material|SetMaterial _sm_kitchen_door_2 0 "/Game/HouseProject/House/Materials/wallpaper/M_wallpaper_051.M_wallpaper_051"))
      (:Out%207
        (Rendering|Material|SetMaterial _sm_kitchen_door_2 0 "/Game/HouseProject/House/Materials/wallpaper/M_wallpaper_050.M_wallpaper_050"))
      (:Out%208
        (Rendering|Material|SetMaterial _sm_kitchen_door_2 0 "/Game/HouseProject/House/Materials/wallpaper/M_wallpaper_048.M_wallpaper_048"))
      (:Out%209
        (Rendering|Material|SetMaterial _sm_kitchen_door_2 0 "/Game/HouseProject/House/Materials/wallpaper/M_wallpaper_018_3.M_wallpaper_018_3"))
      (:Out%2010
        (Rendering|Material|SetMaterial _sm_kitchen_door_2 0 "/Game/HouseProject/House/Materials/wallpaper/M_wallpaper_040.M_wallpaper_040"))
      (:Out%2011
        (Rendering|Material|SetMaterial _sm_kitchen_door_2 0 "/Game/HouseProject/House/Materials/wallpaper/M_wallpaper_036.M_wallpaper_036"))
      (:Out%2012
        (Rendering|Material|SetMaterial _sm_kitchen_door_2 0 "/Game/HouseProject/House/Materials/wallpaper/M_wallpaper_027.M_wallpaper_027"))
      (:Out%2013
        (Rendering|Material|SetMaterial _sm_kitchen_door_2 0 "/Game/HouseProject/House/Materials/Color/M_mat070.M_mat070"))
      (:Out%2014
        (Rendering|Material|SetMaterial _sm_kitchen_door_2 0 "/Game/HouseProject/House/Materials/Color/M_color1.M_color1"))
      (:Out%2015
        (Rendering|Material|SetMaterial _sm_kitchen_door_2 0 "/Game/HouseProject/House/Materials/Color/M_color2.M_color2"))
      (:Out%2016
        (Rendering|Material|SetMaterial _sm_kitchen_door_2 0 "/Game/HouseProject/House/Materials/Color/M_color3.M_color3"))
      (:Out%2017
        (Rendering|Material|SetMaterial _sm_kitchen_door_2 0 "/Game/HouseProject/House/Materials/Color/M_color4.M_color4"))
      (:Out%2018
        (Rendering|Material|SetMaterial _sm_kitchen_door_2 0 "/Game/HouseProject/House/Materials/Color/M_color5.M_color5")))))

(fn ConstructionScript)